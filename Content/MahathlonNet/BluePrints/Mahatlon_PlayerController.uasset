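; Player controller for Mahathlon that lets the player switch control between the units of squad A.
; On BeginPlay it has the GameInstance spawn squad A, possesses its current unit, shows the main menu through a widget message, then spawns squad B.
; Next and Prev inputs step a wrapping index through the squad A array and possess that unit.
; The Main Menu input reopens the menu; the local CreateAndShowWidget function is an empty stub.
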(event EventBeginPlay
  ;[1 0.7031 0.9387] INITIALIZING
  (Development|PrintString "PC Loaded" true true "(R=0.000000,G=0.660000,B=1.000000,A=1.000000)" 1e+01)
  (bind _asmahatthlon_game_instance (Utilities|Casting|CastToMahatthlon_GameInstance (Game|GetGameInstance)))
  (bind _output_get (Variables|Default|SetAs%20Mahatthlon%20Game%20Instance _asmahatthlon_game_instance))
  ;[1 0.7031 0.9387] INIT SPAWN (ON BASE)
  (Default|SpawnASquad _output_get)
  (bind _output_get_2 (Variables|Default|SetCurrent%20Unit%20ref (Variables|/Game/MahathlonNet/BluePrints/Mahatthlon_GameInstance.Mahatthlon_GameInstance_C|GetCurrent_Unit _output_get)))
  (Pawn|Possess _output_get_2)
  ;[1 0.7031 0.9387] INIT SHOW MAIN MENU
  (Class|GameInstanceInterface|CreateandShowWidget(Message) (Game|GetGameInstance) "/Game/MahathlonNet/UI/MainMenu_WBP.MainMenu_WBP_C" "NewEnumerator1" true)
  ;[1 0.7031 0.9387] MAX UNITS AMOUNT
  (Variables|Default|SetUnits%20Amount (Utilities|Array|Length (Variables|/Game/MahathlonNet/BluePrints/Mahatthlon_GameInstance.Mahatthlon_GameInstance_C|GetA_Squad_Array (Variables|Default|GetAs%20Mahatthlon%20Game%20Instance))))
  (Default|SpawnBSquad (Variables|Default|GetAs%20Mahatthlon%20Game%20Instance)))

(event Input|ActionEvents|InputActionNextUnit
  (params (Key :type Key%20Structure :default "None"))
  ;[1 1 1] NEXT/PREV UNIT
  (:Pressed
    (bind _result (Math|Integer|IncrementInt (Variables|Default|GetCurrent%20Unit%20Index))
      (:%20%20
        (if (> _result (- (Variables|Default|GetUnits%20Amount) 1))
          (Variables|Default|SetCurrent%20Unit%20Index 0))
        (bind _output_get (Variables|Default|SetCurrent%20Unit%20ref (Utilities|Array|Get(acopy) (Variables|/Game/MahathlonNet/BluePrints/Mahatthlon_GameInstance.Mahatthlon_GameInstance_C|GetA_Squad_Array (Variables|Default|GetAs%20Mahatthlon%20Game%20Instance)) (Variables|Default|GetCurrent%20Unit%20Index))))
        (Pawn|Possess _output_get)))))

(event Input|ActionEvents|InputActionPrevUnit
  (params (Key :type Key%20Structure :default "None"))
  ;[1 1 1] NEXT/PREV UNIT
  (:Pressed
    (bind _result (Math|Integer|DecrementInt (Variables|Default|GetCurrent%20Unit%20Index))
      (:%20%20
        (if (< _result 0)
          (Variables|Default|SetCurrent%20Unit%20Index (- (Variables|Default|GetUnits%20Amount) 1)))
        (bind _output_get (Variables|Default|SetCurrent%20Unit%20ref (Utilities|Array|Get(acopy) (Variables|/Game/MahathlonNet/BluePrints/Mahatthlon_GameInstance.Mahatthlon_GameInstance_C|GetA_Squad_Array (Variables|Default|GetAs%20Mahatthlon%20Game%20Instance)) (Variables|Default|GetCurrent%20Unit%20Index))))
        (Pawn|Possess _output_get)))))

(event Input|ActionEvents|InputActionMainMenu
  (params (Key :type Key%20Structure :default "None"))
  ;[1 1 1] SHOW MAIN  MENU
  (:Pressed
    (bind _shown_widget (Class|GameInstanceInterface|CreateandShowWidget(Message) (Game|GetGameInstance) "/Game/MahathlonNet/UI/MainMenu_WBP.MainMenu_WBP_C" "NewEnumerator1" true))
    (Variables|Default|SetCreated%20Widget _shown_widget)))

(fn ConstructionScript)

(fn CreateandShowWidget
  (params (Widget%20To%20Show :type Widget%20Class%20Reference) (NewParam :type Input_Modes_Enum%20Enum :default "NewEnumerator0") (Show%20Mousw%20Cursor :type Boolean))
  (return 0))
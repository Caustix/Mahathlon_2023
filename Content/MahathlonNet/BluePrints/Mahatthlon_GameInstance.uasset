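; Game instance for Mahathlon that spawns both player squads and provides shared widget and quit helpers.
; SpawnUnits reads side A or B squad structs from GameMod_Server, spawns units at that side's player starts by index, copies identity and action points, and zeroes health.
; Each squad fills its own array, with the first unit set as current.
; Widget helpers show or hide UI while setting cursor visibility and input mode.
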(event Custom|Spawn%20A_Squad
  (CallFunction|SpawnUnits "NewEnumerator0"))

(event Custom|Spawn%20B_Squad
  (CallFunction|SpawnUnits "NewEnumerator3"))

(event EventQuitGame
  (Game|QuitGame 0 "Quit" false))

(fn CreateandShowWidget
  (params (Widget%20To%20Show :type User%20Widget%20Class%20Reference) (NewParam :type Input_Modes_Enum%20Enum :default "NewEnumerator0") (Show%20Mousw%20Cursor :type Boolean))
  (Variables|References|SetCreated%20Widget 0)
  (bind _asmahatlon_player_controller (Utilities|Casting|CastToMahatlon_PlayerController (Game|GetPlayerController 0)))
  (bind _output_get (Variables|References|SetAs%20Mahatlon%20Player%20Controller _asmahatlon_player_controller))
  (Variables|/Script/Engine.PlayerController|SetbShowMouseCursor _output_get Show%20Mousw%20Cursor)
  (Utilities|IsValid (Variables|References|GetCreated%20Widget)
    (:Is%20Valid
      _)
    (:Is%20Not%20Valid
      (bind _returnvalue (UserInterface|CreateWidget Widget%20To%20Show (Variables|References|GetAs%20Mahatlon%20Player%20Controller)))
      (bind _output_get_2 (Variables|References|SetCreated%20Widget _returnvalue))))
  (UserInterface|Viewport|AddtoViewport _output_get_2 0)
  (switch Utilities|FlowControl|Switch|SwitchonInput_Modes_Enum NewParam
    (:NewEnumerator0
      (Input|SetInputModeGameOnly (Variables|References|GetAs%20Mahatlon%20Player%20Controller)))
    (:NewEnumerator1
      (Input|SetInputModeUIOnly (Variables|References|GetAs%20Mahatlon%20Player%20Controller) (Variables|References|GetCreated%20Widget) "LockInFullscreen"))
    (:NewEnumerator2
      (Input|SetInputModeGameandUI (Variables|References|GetAs%20Mahatlon%20Player%20Controller) (Variables|References|GetCreated%20Widget) "LockInFullscreen" true))
    (:NewEnumerator3
      _))
  (return (Variables|References|GetCreated%20Widget)))

(fn HideWidget
  (params (Widget%20to%20Hide :type Widget%20Object%20Reference) (Show%20Mouse%20Cursor :type Boolean) (Input%20mode :type Input_Modes_Enum%20Enum :default "NewEnumerator0"))
  (bind _created_widget (Variables|References|GetCreated%20Widget))
  (Widget|RemovefromParent Widget%20to%20Hide)
  (bind _asmahatlon_player_controller (Utilities|Casting|CastToMahatlon_PlayerController (Game|GetPlayerController 0)))
  (bind _output_get (Variables|References|SetAs%20Mahatlon%20Player%20Controller _asmahatlon_player_controller))
  (Variables|/Script/Engine.PlayerController|SetbShowMouseCursor _output_get Show%20Mouse%20Cursor)
  (switch Utilities|FlowControl|Switch|SwitchonInput_Modes_Enum Input%20mode
    (:NewEnumerator0
      (Input|SetInputModeGameOnly (Variables|References|GetAs%20Mahatlon%20Player%20Controller))
      (return))
    (:NewEnumerator1
      (Input|SetInputModeUIOnly (Variables|References|GetAs%20Mahatlon%20Player%20Controller) _created_widget "LockInFullscreen"))
    (:NewEnumerator2
      (Input|SetInputModeGameandUI (Variables|References|GetAs%20Mahatlon%20Player%20Controller) _created_widget "LockInFullscreen" true)
      (return))
    (:NewEnumerator3
      (return))))

(fn SpawnUnits
  (params (Player%20Starts :type Player_Side_Enum1%20Enum :default "NewEnumerator0"))
  (bind _asgame_mod_server (Utilities|Casting|CastToGameMod_Server (Game|GetGameMode)))
  (Variables|References|SetAs%20Game%20Mod%20Server _asgame_mod_server)
  (switch Utilities|FlowControl|Switch|SwitchonPlayer_Side_Enum1 Player%20Starts
    (:NewEnumerator0
      (bind _outactors (Actor|GetAllActorsOfClass "/Game/MahathlonNet/BluePrints/A_PayerStartBP.A_PayerStartBP_C"))
      (Variables|Default|SetA_PlayerStarts _outactors)
      ;[1 1 1] Spawning A Squad
      (for (_array_element _array_index) (Variables|/Game/MahathlonNet/BluePrints/GameMod_Server.GameMod_Server_C|GetA_Squad_Struct_Array (Variables|References|GetAs%20Game%20Mod%20Server))
        (LocalVariables|SetCurrent%20Unit%20From%20Server _array_element)
        (bind _returnvalue (Game|SpawnActorfromClass "/Game/MahathlonNet/BluePrints/A_BAseUnitBP.A_BAseUnitBP_C" (Transformation|GetActorTransform (Utilities|Array|Get(acopy) (Variables|Default|GetA_PlayerStarts) _array_index)) "AlwaysSpawn" (Variables|References|GetAs%20Mahatlon%20Player%20Controller) 0))
        (bind _output_get (Variables|Default|SetCurrent_Unit _returnvalue))
        (Variables|/Game/MahathlonNet/BluePrints/BaseUnitBP.BaseUnitBP_C|SetPortrait _output_get (.portrait (LocalVariables|GetCurrent%20Unit%20From%20Server)))
        (Variables|/Game/MahathlonNet/BluePrints/BaseUnitBP.BaseUnitBP_C|SetName _output_get (.name (LocalVariables|GetCurrent%20Unit%20From%20Server)))
        (Variables|/Game/MahathlonNet/BluePrints/BaseUnitBP.BaseUnitBP_C|SetSurname _output_get (.surname (LocalVariables|GetCurrent%20Unit%20From%20Server)))
        (Variables|/Game/MahathlonNet/BluePrints/BaseUnitBP.BaseUnitBP_C|SetAction%20Points _output_get (.actionpoints (LocalVariables|GetCurrent%20Unit%20From%20Server)))
        (Variables|/Game/MahathlonNet/BluePrints/BaseUnitBP.BaseUnitBP_C|SetHealth%20Points _output_get 0)
        (Utilities|Array|Add (Variables|Default|GetA_Squad_Array) _output_get))
      (Variables|Default|SetCurrent_Unit (Utilities|Array|Get(acopy) (Variables|Default|GetA_Squad_Array)))
      (return true))
    (:NewEnumerator3
      (bind _outactors_2 (Actor|GetAllActorsOfClass "/Game/MahathlonNet/BluePrints/B_PayerStartBP.B_PayerStartBP_C"))
      (Variables|Default|SetB_PlayerStarts _outactors_2)
      ;[1 1 1] Spawning B Squad
      (for (_array_element_2 _array_index_2) (Variables|/Game/MahathlonNet/BluePrints/GameMod_Server.GameMod_Server_C|GetB_Squad_Struct_Array (Variables|References|GetAs%20Game%20Mod%20Server))
        (LocalVariables|SetCurrent%20Unit%20From%20Server _array_element_2)
        (bind _returnvalue_2 (Game|SpawnActorfromClass "/Game/MahathlonNet/BluePrints/B_BAseUnitBP.B_BAseUnitBP_C" (Transformation|GetActorTransform (Utilities|Array|Get(acopy) (Variables|Default|GetB_PlayerStarts) _array_index_2)) "AlwaysSpawn" (Variables|References|GetAs%20Mahatlon%20Player%20Controller) 0))
        (bind _output_get_2 (Variables|Default|SetCurrent_Unit _returnvalue_2))
        (Variables|/Game/MahathlonNet/BluePrints/BaseUnitBP.BaseUnitBP_C|SetPortrait _output_get_2 (.portrait (LocalVariables|GetCurrent%20Unit%20From%20Server)))
        (Variables|/Game/MahathlonNet/BluePrints/BaseUnitBP.BaseUnitBP_C|SetName _output_get_2 (.name (LocalVariables|GetCurrent%20Unit%20From%20Server)))
        (Variables|/Game/MahathlonNet/BluePrints/BaseUnitBP.BaseUnitBP_C|SetSurname _output_get_2 (.surname (LocalVariables|GetCurrent%20Unit%20From%20Server)))
        (Variables|/Game/MahathlonNet/BluePrints/BaseUnitBP.BaseUnitBP_C|SetAction%20Points _output_get_2 (.actionpoints (LocalVariables|GetCurrent%20Unit%20From%20Server)))
        (Variables|/Game/MahathlonNet/BluePrints/BaseUnitBP.BaseUnitBP_C|SetHealth%20Points _output_get_2 0)
        (Utilities|Array|Add (Variables|Default|GetB_Squad_Array) _output_get_2))
      (Variables|Default|SetCurrent_Unit (Utilities|Array|Get(acopy) (Variables|Default|GetB_Squad_Array)))
      (return true))))